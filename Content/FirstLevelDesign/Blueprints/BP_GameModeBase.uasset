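; Game mode Blueprint that respawns the player character whenever it is destroyed.
; On BeginPlay it binds to the OnDestroyed event of the current BP_Character.
; When that fires, it waits briefly, spawns a new BP_Character at the SpawnTransform variable and has the first player controller possess it.
; It then calls Respawn to bind the new character, keeping the cycle going.
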(event `Respawn`
  (bind _asbp_character (cast `/Game/FirstLevelDesign/Blueprints/BP_Character` (`GameplayStatics.GetPlayerCharacter` 0) :!label _label))
  (add `self.OnDestroyed` _asbp_character (delegate `OnDestroyed_`)))

(event `self.ReceiveBeginPlay`
  (goto _label))

(event `OnDestroyed_` :!signature `self.OnDestroyed`
  (params (DestroyedActor :type "Actor Object Reference"))
  (`KismetSystemLibrary.Delay` 0.2)
  (bind _returnvalue (`|SpawnActorFromClass` "/Game/FirstLevelDesign/Blueprints/BP_Character.BP_Character_C" (`self.Spawn Transform`) "Undefined" "OverrideRootScale" null null))
  (`Controller.Possess` (`GameplayStatics.GetPlayerController` 0) _returnvalue)
  (`self.Respawn`))

(fn `UserConstructionScript`)