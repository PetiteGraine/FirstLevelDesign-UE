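; Player character Blueprint with Enhanced Input movement, camera look, double jump and death.
; BeginPlay clears IsRecovering after a short delay, then adds the default mapping context; CanMove blocks movement while dead or recovering.
; The double jump switches a falling character to Walking before calling Jump, and landing re-arms it.
; Die plays the death animation and sets IsDead.
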(event `self.ReceiveBeginPlay`
  ;[1 1 1] Mapping Context
  (`KismetSystemLibrary.Delay` 0.75)
  (set `self.isRecovering` false)
  (bind _asplayer_controller (cast `PlayerController` (`self.GetController`)))
  (bind _returnvalue (pcsubsystem `EnhancedInputLocalPlayerSubsystem` _asplayer_controller))
  (`/Engine/EditorBlueprintResources/StandardMacros.IsValid` _returnvalue
    (:`Is Valid`
      (`EnhancedInputSubsystemInterface.AddMappingContext` _returnvalue "/Game/FirstLevelDesign/Input/IMC_Default.IMC_Default" 0 (struct)))))

(event `EnhancedInput|/Game/FirstLevelDesign/Input/Actions/IA_Move`
  (params (ActionValue :type "Vector2D Structure") (ElapsedSeconds :type "Float (double-precision)") (TriggeredSeconds :type "Float (double-precision)") (InputAction :type "InputAction Object Reference" :default "/Game/FirstLevelDesign/Input/Actions/IA_Move.IA_Move"))
  (bind (_returnvalue_roll _returnvalue_pitch _returnvalue_yaw) (`KismetMathLibrary.BreakRotator` (`self.GetControlRotation`)))
  (bind _returnvalue (`KismetMathLibrary.MakeRotator` 0.0 0.0 _returnvalue_yaw))
  ;[1 1 1] Movement
  (:`Triggered`
    (bind _canmove (`self.CanMove_`))
    (if _canmove
      (`self.AddMovementInput` (`KismetMathLibrary.GetForwardVector` _returnvalue) ActionValue_X)
      (`self.AddMovementInput` (`KismetMathLibrary.GetRightVector` _returnvalue) ActionValue_Y))))

(event `EnhancedInput|/Game/FirstLevelDesign/Input/Actions/IA_Look`
  (params (ActionValue :type "Vector2D Structure") (ElapsedSeconds :type "Float (double-precision)") (TriggeredSeconds :type "Float (double-precision)") (InputAction :type "InputAction Object Reference" :default "/Game/FirstLevelDesign/Input/Actions/IA_Look.IA_Look"))
  ;[1 1 1] Camera
  (:`Triggered`
    (`self.AddControllerYawInput` ActionValue_X)
    (`self.AddControllerPitchInput` (* ActionValue_Y -1.0))))

(event `EnhancedInput|/Game/FirstLevelDesign/Input/Actions/IA_Jump`
  (params (ActionValue :type Boolean) (ElapsedSeconds :type "Float (double-precision)") (TriggeredSeconds :type "Float (double-precision)") (InputAction :type "InputAction Object Reference" :default "/Game/FirstLevelDesign/Input/Actions/IA_Jump.IA_Jump"))
  (bind _charactermovement (`self.CharacterMovement`))
  ;[1 1 1] Double Jump
  (:`Started`
    (bind _canmove (`self.CanMove_`))
    (if (and _canmove (`self.Can Double Jump`) (`NavMovementComponent.IsFalling` (`self.CharacterMovement`)))
      (set `CharacterMovementComponent.JumpOffJumpZFactor` 600.0 _charactermovement)
      (`CharacterMovementComponent.SetMovementMode` _charactermovement "MOVE_Walking" 0)
      (set `self.Can Double Jump` false)
      (else
        (set `CharacterMovementComponent.JumpOffJumpZFactor` 700.0 _charactermovement)))
    (`self.Jump`)
    (if (`|EnumInequality` (`CharacterMovementComponent.MovementMode` (`self.CharacterMovement`)) "MOVE_Falling")
      (`GameplayStatics.PlaySoundAtLocation` "/Game/HumanVocalizations/HumanMaleC/Cues/voice_male_c_effort_short_jump_01_Cue.voice_male_c_effort_short_jump_01_Cue" (`self.K2_GetActorLocation`) (struct) 1.0 1.0 0.0 null null null null)))
  (:`Completed`
    (`self.StopJumping`)))

(event `self.OnLanded`
  (params (Hit :type "HitResult Structure (by ref)"))
  ;[1 1 1] Double Jump
  (set `self.Can Double Jump` true))

(fn `CanMove_`
  (returns (CanMove :type Boolean))
  (return (`KismetMathLibrary.BooleanNOR` (`self.isDead`) (`self.isRecovering`))))

(fn `Die`
  (`SkeletalMeshComponent.PlayAnimation` (`self.Mesh`) "/Game/BattleWizardPolyart/Animations/DieAnim.DieAnim" false)
  (set `self.isDead` true))

(fn `UserConstructionScript`)