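; BP_Teleporter_A is a placeable teleporter that moves any actor entering its box to a TeleportLocation transform.
; On overlap it sets the actor's root transform, plays a teleport sound, and for BP_Character also aligns control rotation to the new facing and adds a pitch input.
; The construction script places an Arrow component at the destination, previewing where and which way actors arrive.
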(event `self.Box.OnComponentBeginOverlap`
  (params (OverlappedComponent :type "PrimitiveComponent Object Reference") (OtherActor :type "Actor Object Reference") (OtherComp :type "PrimitiveComponent Object Reference") (OtherBodyIndex :type Integer) (bFromSweep :type Boolean) (SweepResult :type "HitResult Structure (by ref)"))
  (`SceneComponent.K2_SetWorldTransform` (`Actor.RootComponent` OtherActor) (`self.Teleport Location`) false true)
  (`GameplayStatics.PlaySoundAtLocation` "/Game/FirstLevelDesign/Sounds/Teleport.Teleport" (`self.K2_GetActorLocation` OtherActor) (struct) 1.0 1.0 0.0 null null null null)
  (bind _asbp_character (cast `/Game/FirstLevelDesign/Blueprints/BP_Character` OtherActor))
  (`Controller.SetControlRotation` (`Pawn.GetController` _asbp_character) (`self.K2_GetActorRotation` _asbp_character))
  (`Pawn.AddControllerPitchInput` _asbp_character 10.0))

(fn `UserConstructionScript`
  (`SceneComponent.K2_SetWorldTransform` (`self.Arrow`) (`self.Teleport Location`) false false))